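; BP_Platform is a side-scroller platform that turns solid to pawns again after characters have passed through it.
; When a SideScrollerCharacter stops overlapping PlatformMesh and no others remain inside, the mesh's Pawn collision response is set back to Block.
; The switch to a passable state happens outside this file.
; The construction script snaps the actor to X = 0, keeping Y and Z, so it stays on the gameplay plane.
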(event `self.PlatformMesh.OnComponentEndOverlap`
  (params (OverlappedComponent :type "PrimitiveComponent Object Reference") (OtherActor :type "Actor Object Reference") (OtherComp :type "PrimitiveComponent Object Reference") (OtherBodyIndex :type Integer))
  (cast `/Game/SideScrollerBP/Blueprints/SideScrollerCharacter` OtherActor)
  (if (== (`KismetArrayLibrary.Array_Length` (`PrimitiveComponent.GetOverlappingActors` (`self.PlatformMesh`) "/Game/SideScrollerBP/Blueprints/SideScrollerCharacter.SideScrollerCharacter_C")) 0)
    (`PrimitiveComponent.SetCollisionResponseToChannel` (`self.PlatformMesh`) "ECC_Pawn" "ECR_Block")))

(fn `UserConstructionScript`
  (bind (_returnvalue_x _returnvalue_y _returnvalue_z) (`KismetMathLibrary.BreakVector` (`self.K2_GetActorLocation`)))
  (`self.K2_SetActorLocation` (`KismetMathLibrary.MakeVector` 0.0 _returnvalue_y _returnvalue_z)))